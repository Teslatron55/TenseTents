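; BP_KnifeSnap is a grabbable knife prop that snaps into a motion controller's grip and destroys itself on overlapping a DuckEnemy.
; Pickup, called by BP_MotionController, disables physics, attaches the root to the given component and sets a hard-coded mesh offset and rotation for the held pose.
; Drop re-enables physics and detaches the actor while keeping its world transform.
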(event OnComponentBeginOverlap(StaticMeshComponent)
  (params (OverlappedComponent :type Primitive%20Component%20Object%20Reference) (OtherActor :type Actor%20Object%20Reference) (OtherComp :type Primitive%20Component%20Object%20Reference) (OtherBodyIndex :type Integer) (bFromSweep :type Boolean) (SweepResult :type Hit%20Result%20Structure%20%28by%20ref%29))
  (Utilities|Casting|CastToDuckEnemy OtherActor)
  (Actor|DestroyActor))

(event EventPickup
  (params (AttachTo :type Scene%20Component%20Object%20Reference))
  ;[1 1 1] Picking up, Dropping
  (Physics|SetSimulatePhysics (Variables|Debug|GetStaticMeshComponent) false)
  (Transformation|AttachComponentToComponent (VehicleSound|GetRootComponent) AttachTo "None" "SnapToTarget" "SnapToTarget" "KeepWorld" false)
  (Transformation|SetRelativeLocationAndRotation (Variables|Debug|GetStaticMeshComponent) "-0.015100,0.999900,1.863240" "-80.000000,-126.000000,1115.000000" true false))

(event EventDrop
  ;[1 1 1] Picking up, Dropping
  (Physics|SetSimulatePhysics (Variables|Debug|GetStaticMeshComponent) true)
  (Transformation|DetachFromActor "KeepWorld" "KeepWorld" "KeepWorld"))

(fn ConstructionScript)